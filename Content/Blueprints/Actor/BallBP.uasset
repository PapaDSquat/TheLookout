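; Grabbable, throwable physics ball that shows its grab state to the player and can be respawned.
; Grab, release and range-change events call UpdateMaterial to pick the grabbed, can-grab or default material, with sounds on grab and drop.
; Release also reports the throw to PlayerStateBP, marked as a TODO to move into PlayerPawn.
; Respawn teleports the ball and zeroes its velocity; the wall bounce sound is unconnected.
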(event OnComponentHit(Sphere)
  (params (HitComponent :type Primitive%20Component%20Object%20Reference) (OtherActor :type Actor%20Object%20Reference) (OtherComp :type Primitive%20Component%20Object%20Reference) (NormalImpulse :type Vector :default "0, 0, 0") (Hit :type Hit%20Result%20Structure%20%28by%20ref%29)))

(event EventOnPlayerRelease
  (bind _returnvalue (Game|Player|GetPlayerPawn 0))
  (State|UpdateMaterial)
  (Audio|PlaySoundatLocation "/Game/Audio/sound_ball_drop_cue.sound_ball_drop_cue" (Transformation|GetActorLocation) "0, 0, 0" 1.0 1.0 0.0 0 0 0)
  ;[1 1 1] TODO : Should be done in PlayerPawn on event callback
  (Utilities|IsValid _returnvalue
    (:Is%20Valid
      (bind _asplayer_state_bp (Utilities|Casting|CastToPlayerStateBP (Variables|/Script/Engine.Pawn|GetPlayerState _returnvalue)))
      (Default|OnThrowBall _asplayer_state_bp))))

(event EventOnPlayerGrab
  (State|UpdateMaterial)
  (Audio|PlaySoundatLocation "/Game/Audio/sound_ball_grab_cue.sound_ball_grab_cue" (Transformation|GetActorLocation) "0, 0, 0" 1.0 1.0 0.0 0 0 0))

(event EventOninGrabRangeChange
  (params (inRange :type Boolean))
  (State|UpdateMaterial))

(fn ConstructionScript)

(fn UpdateMaterial
  (if (Variables|Default|GetIsGrabbed)
    (Rendering|Material|SetMaterial (Variables|Default|GetSphere) 0 "/Game/Materials/BallGrabbedMaterial.BallGrabbedMaterial")
    (elif (Class|Ball|InGrabRange)
      (Rendering|Material|SetMaterial (Variables|Default|GetSphere) 0 "/Game/Materials/BallCanGrabMaterial.BallCanGrabMaterial")
      (else
        (Rendering|Material|SetMaterial (Variables|Default|GetSphere) 0 "/Game/Materials/BallDefaultMaterial.BallDefaultMaterial")))))

(fn Respawn
  (params (Location :type Vector))
  (Transformation|Teleport Location "0, 0, 0")
  (Physics|SetPhysicsLinearVelocity (Variables|Default|GetSphere) "0, 0, 0" false "None"))