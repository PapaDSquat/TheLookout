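; A grabbable grenade ball that starts a fuse when the player grabs it and explodes with a radial impulse and sound.
; Tick advances a normalized charge from the remaining fuse time, which scales the explosion sphere and brightens its emission.
; Releasing the ball leaves the fuse running, and exploding stops the charge, which then resets to zero.
; A separate material function varies ball opacity by grab state and range.
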(event Custom|OnExplode
  ;[1 1 1] Push Player on Explode
  (Variables|State|SetIsCharging false)
  (CallFunction|UpdateCurrentTimer)
  (Class|RadialForceComponent|FireImpulse (Variables|Default|GetRadialForce))
  (Audio|PlaySoundatLocation "/Game/Audio/sound_explosion_cue.sound_explosion_cue" (Transformation|GetActorLocation) "0, 0, 0" 3.0 1.0 0.0 0 0 0))

(event EventTick
  (params (DeltaSeconds :type Float%20%28single-precision%29))
  (bind _sphere (Variables|Default|GetSphere))
  (bind _currentcharge (Variables|State|GetCurrentCharge))
  (bind _returnvalue (Transformation|GetWorldScale _sphere))
  (bind _returnvalue_2 (* (.x _returnvalue) _currentcharge))
  (|CallParentFunction DeltaSeconds)
  (CallFunction|UpdateCharge DeltaSeconds)
  (Transformation|SetWorldScale3D (Variables|Default|GetExplosionSphere) (Math|Vector|MakeVector _returnvalue_2 _returnvalue_2 _returnvalue_2)) ; Set Explosion Sphere Scale
  (CallFunction|UpdateExplodeMaterial))

(event EventOnPlayerGrab
  (|CallParentFunction)
  (Variables|State|SetIsCharging true)
  (CallFunction|UpdateCurrentTimer))

(event EventOnPlayerRelease
  (|CallParentFunction))

(fn ConstructionScript
  (|CallParentFunction))

(fn UpdateCharge
  (params (DeltaTime :type Float%20%28single-precision%29))
  (if (Variables|State|GetIsCharging)
    (if (> (Variables|State|GetCurrentTime) 0.0)
      (Variables|State|SetCurrentTime (Math|Float|Max(Float) (- (Variables|State|GetCurrentTime) DeltaTime) 0.0))
      (Utilities|FlowControl|Sequence
        (:then_0
          ;[1 1 1] Update Current Charge [0.0, 1.0]
          (Variables|State|SetCurrentCharge (- 1.0 (/ (Variables|State|GetCurrentTime) (Variables|GrenadeSettings|GetTimeToExplode))))
          (if (== (Variables|State|GetCurrentTime) 0.0)
            (CallFunction|OnExplode)))))
    (else
      (Variables|State|SetCurrentCharge 0.0))))

(fn UpdateExplodeMaterial
  (Rendering|Material|SetScalarParameterValueonMaterials (Variables|Default|GetExplosionSphere) "Emission" (Math|Float|Lerp 2.5e+02 6e+02 (Variables|State|GetCurrentCharge))))

(fn UpdateCurrentTimer
  (Variables|State|SetCurrentTime (* (- 1.0 (Variables|State|GetCurrentCharge)) (Variables|GrenadeSettings|GetTimeToExplode))))

(fn UpdateMaterial
  (if (Variables|Default|GetIsGrabbed)
    (Rendering|Material|SetScalarParameterValueonMaterials (Variables|Default|GetSphere) "Opacity" 0.4)
    (elif (Class|Ball|InGrabRange)
      (Rendering|Material|SetScalarParameterValueonMaterials (Variables|Default|GetSphere) "Opacity" 0.9)
      (else
        (Rendering|Material|SetScalarParameterValueonMaterials (Variables|Default|GetSphere) "Opacity" 0.7)))))