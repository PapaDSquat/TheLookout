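; Physics-simulated target actor for the hide-and-seek game that reacts to Ball hits.
; On game start from HideAndSeekGameState, it teleports back to its BeginPlay transform, pausing physics to do so, and re-arms.
; The first Ball hit while active plays a bounce sound and latches TargetHit.
; A separate OnTargetHit event deactivates the target, swapping the cube's pulsing material for a static one; nothing here calls it.
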(event Custom|OnTargetHit
  (State|SetTargetActive false))

(event Custom|OnGameStart
  (State|RespawnTarget)
  (State|SetTargetActive true)
  (Variables|State|SetTargetHit false))

(event EventBeginPlay
  (bind _gamestate (Helpers|GetHideandSeekGameState))
  (State|SetTargetActive true)
  (Variables|Cache|SetInitialTransform (Transformation|GetActorTransform))
  (Utilities|IsValid _gamestate
    (:Is%20Valid
      (EventDispatchers|BindEventtoOnGameStart _gamestate (delegate Custom|OnGameStart)))))

(event Collision|EventHit
  (params (MyComp :type Primitive%20Component%20Object%20Reference) (Other :type Actor%20Object%20Reference) (OtherComp :type Primitive%20Component%20Object%20Reference) (bSelfMoved :type Boolean) (HitLocation :type Vector :default "0, 0, 0") (HitNormal :type Vector :default "0, 0, 0") (NormalImpulse :type Vector :default "0, 0, 0") (Hit :type Hit%20Result%20Structure%20%28by%20ref%29))
  (Utilities|Casting|CastToBall Other)
  (if (Variables|State|GetTargetActive)
    (if (not (Variables|State|GetTargetHit))
      (Audio|PlaySoundatLocation "/Game/Audio/sound_bounce01.sound_bounce01" (Transformation|GetActorLocation) "0, 0, 0" 1.0 1.0 0.0 0 0 0)
      (Variables|State|SetTargetHit true))))

(fn ConstructionScript)

(fn SetTargetActive
  (params (Value :type Boolean))
  (bind _cube (Variables|Default|GetCube))
  (bind _output_get (Variables|State|SetTargetActive Value))
  (if _output_get
    (Rendering|Material|SetMaterial _cube 0 "/Game/StarterContent/Materials/M_Tech_Hex_Tile_Pulse.M_Tech_Hex_Tile_Pulse")
    (else
      (Rendering|Material|SetMaterial _cube 0 "/Game/StarterContent/Materials/M_Tech_Hex_Tile.M_Tech_Hex_Tile"))))

(fn GetHideandSeekGameState
  (bind _ashide_and_seek_game_state (Utilities|Casting|CastToHideAndSeekGameState (Game|GetGameState))
    (:then
      (return _ashide_and_seek_game_state))
    (:CastFailed
      (return 0))))

(fn RespawnTarget
  (bind _initialtransform (Variables|Cache|GetInitialTransform))
  (bind _cube (Variables|Default|GetCube))
  (Physics|SetPhysicsLinearVelocity _cube "0, 0, 0" false "None")
  (Physics|SetSimulatePhysics _cube false)
  (Transformation|SetActorRotation (.rotation _initialtransform) true)
  (Transformation|SetActorLocation (.location _initialtransform) false true)
  (Physics|SetSimulatePhysics _cube true))