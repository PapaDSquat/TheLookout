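; Game mode for a timed hide-and-seek game where player 0 scores by hitting targets with thrown balls.
; On login it spawns and possesses a VR lookout for the first player and agent characters for the next three, using tagged PlayerStarts.
; It counts targets, respawns balls at random spawners, and ends on timeout or all targets hit.
; Final score combines hits, all-target bonus, time left and a bonus reduced per throw.
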(event Custom|OnTargetHit
  (params (TargetActor :type Target%20Actor%20BP%20Object%20Reference))
  (Utilities|IsValid TargetActor
    (:Is%20Valid
      (PublicInterface|AddPoint))))

(event Custom|OnTimeRunOut
  (PublicInterface|EndGame))

(event EventBeginPlay
  (bind _gamestate (Helpers|GetHideandSeekGameState))
  (Utilities|FlowControl|Sequence
    (:then_0
      (bind _outactors (Actor|GetAllActorsOfClass "/Game/Blueprints/Actor/TargetActorBP.TargetActorBP_C"))
      (Variables|GameParams|SetTotalTargets (Utilities|Array|Length _outactors)))
    (:then_1
      (bind _outactors_2 (Actor|GetAllActorsOfClass "/Game/Blueprints/Actor/BallSpawnerBP.BallSpawnerBP_C"))
      (Variables|Default|SetBallSpawners _outactors_2))
    (:then_2
      (Utilities|IsValid _gamestate
        (:Is%20Valid
          (EventDispatchers|BindEventtoOnTimeRunOut _gamestate (delegate Custom|OnTimeRunOut)))))))

(event EventPostLogin
  (params (NewPlayer :type Player%20Controller%20Object%20Reference))
  (CallFunction|SpawnPlayers NewPlayer))

(fn ConstructionScript)

(fn AddPoint
  (bind _gamestate (Helpers|GetHideandSeekGameState))
  (bind _gamestate_2 (Helpers|GetHideandSeekPlayerState))
  (Utilities|IsValid _gamestate
    (:Is%20Valid
      (LocalVariables|SetLGameState _gamestate)
      (Utilities|IsValid _gamestate_2
        (:Is%20Valid
          (LocalVariables|SetLPlayerState _gamestate_2)
          (Utilities|FlowControl|Sequence
            (:then_0
              (bind _totalpoints (Default|ScorePoint (LocalVariables|GetLPlayerState)))
              (if (>= _totalpoints (Variables|GameParams|GetTotalTargets))
                (PublicInterface|EndGame)))
            (:then_1
              (Audio|PlaySound2D "/Game/Audio/sound_score01_Cue.sound_score01_Cue" 1.0 1.0 0.0 0 0))))))))

(fn GetTargetsRemaining
  (params (PlayerIndex :type Integer))
  (bind _gamestate (Helpers|GetHideandSeekPlayerState))
  (Utilities|IsValid _gamestate
    (:Is%20Valid
      (return (- (Variables|GameParams|GetTotalTargets) (Variables|/Game/Blueprints/Player/PlayerStateBP.PlayerStateBP_C|GetGamePoints _gamestate))))
    (:Is%20Not%20Valid
      (return -1))))

(fn GetHideandSeekGameState
  (bind _ashide_and_seek_game_state (Utilities|Casting|CastToHideAndSeekGameState (Game|GetGameState))
    (:then
      (return _ashide_and_seek_game_state))
    (:CastFailed
      (return 0))))

(fn GetHideandSeekPlayerState
  (params (PlayerIndex :type Integer))
  (bind _returnvalue (Game|Player|GetPlayerPawn PlayerIndex))
  (Utilities|IsValid _returnvalue
    (:Is%20Valid
      (bind _asplayer_state_bp (Utilities|Casting|CastToPlayerStateBP (Variables|/Script/Engine.Pawn|GetPlayerState _returnvalue))
        (:then
          (return _asplayer_state_bp))
        (:CastFailed
          _)))
    (:Is%20Not%20Valid
      _))
  (return 0))

(fn RespawnBall
  (params (Ball :type Ball%20BP%20Object%20Reference))
  (bind _ballspawners (Variables|Default|GetBallSpawners))
  (bind _outitem (Utilities|Array|Random _ballspawners))
  (Utilities|IsValid _outitem
    (:Is%20Valid
      (Default|Respawn Ball (Transformation|GetActorLocation _outitem)))))

(fn StartGame
  (bind _gamestate (Helpers|GetHideandSeekPlayerState))
  (bind _gamestate_2 (Helpers|GetHideandSeekGameState))
  (if (not (Variables|/Script/TheLookout.TheLookoutGameStateBase|GetGameActive (Helpers|GetHideandSeekGameState)))
    (Utilities|FlowControl|Sequence
      (:then_0
        (Utilities|IsValid _gamestate_2
          (:Is%20Valid
            (Default|RestartGame _gamestate_2 (Variables|GameParams|GetTotalTimeSeconds)))))
      (:then_1
        (Utilities|IsValid _gamestate
          (:Is%20Valid
            (Default|ResetGameStats _gamestate)))))))

(fn EndGame
  (bind _gamestate (Helpers|GetHideandSeekPlayerState))
  (bind _gamestate_2 (Helpers|GetHideandSeekGameState))
  (Utilities|IsValid _gamestate_2
    (:Is%20Valid
      (if (Variables|/Script/TheLookout.TheLookoutGameStateBase|GetGameActive _gamestate_2)
        (Default|EndGame _gamestate_2)
        (Utilities|IsValid _gamestate
          (:Is%20Valid
            (Default|SetFinalGameScore _gamestate (.ScoreTotal (PublicInterface|GetGameScoreBreakdown)))))))))

(fn GetGameScoreBreakdown
  (params (PlayerIndex :type Integer))
  (bind _gamestate (Helpers|GetHideandSeekPlayerState PlayerIndex))
  (bind _gamestate_2 (Helpers|GetHideandSeekGameState))
  (bind _totaltargets (Variables|GameParams|GetTotalTargets))
  (bind _scorebonusforminthrownballs (Variables|Scoring|GetScoreBonusForMinThrownBalls))
  (bind _scorededucterforeachthrownball (Variables|Scoring|GetScoreDeducterForEachThrownBall))
  (bind _scorepertargethit (Variables|Scoring|GetScorePerTargetHit))
  (bind _scorebonusforalltargetshit (Variables|Scoring|GetScoreBonusForAllTargetsHit))
  (bind _scorepersecondleft (Variables|Scoring|GetScorePerSecondLeft))
  (bind _gamepoints (Variables|/Game/Blueprints/Player/PlayerStateBP.PlayerStateBP_C|GetGamePoints _gamestate))
  (bind _timeremaining (Variables|/Game/Blueprints/GameMode/HideAndSeekGameState.HideAndSeekGameState_C|GetTimeRemaining _gamestate_2))
  (bind _ballsthrown (Variables|/Game/Blueprints/Player/PlayerStateBP.PlayerStateBP_C|GetBallsThrown _gamestate))
  (bind _gamepoints_2 (Variables|/Game/Blueprints/Player/PlayerStateBP.PlayerStateBP_C|GetGamePoints _gamestate))
  (bind _returnvalue (>= _gamepoints_2 _totaltargets))
  (bind _returnvalue_2 (Math|Float|Truncate _timeremaining))
  (bind _returnvalue_3 (* _gamepoints _scorepertargethit))
  (bind _returnvalue_4 (* _ballsthrown _scorededucterforeachthrownball))
  (bind _returnvalue_5 (Math|Conversions|ToInteger(Boolean) _returnvalue))
  (bind _returnvalue_6 (- _scorebonusforminthrownballs _returnvalue_4))
  (bind _returnvalue_7 (* _returnvalue_2 _scorepersecondleft))
  (bind _returnvalue_8 (* _returnvalue_5 _scorebonusforalltargetshit))
  (bind _returnvalue_9 (Math|Integer|Max(Integer) _returnvalue_6))
  (bind _returnvalue_10 (+ _returnvalue_3 _returnvalue_8))
  (Utilities|IsValid _gamestate_2
    (:Is%20Valid
      (Utilities|IsValid _gamestate
        (:Is%20Valid
          (if (Variables|/Script/TheLookout.TheLookoutGameStateBase|GetGameJustPlayed _gamestate_2)
            (return _returnvalue (Variables|/Game/Blueprints/GameMode/HideAndSeekGameState.HideAndSeekGameState_C|GetTimeRemaining _gamestate_2) (Variables|GameParams|GetTotalTimeSeconds) (Variables|/Game/Blueprints/Player/PlayerStateBP.PlayerStateBP_C|GetGamePoints _gamestate) (Variables|GameParams|GetTotalTargets) _returnvalue_10 _returnvalue_7 _returnvalue_9 (+ _returnvalue_10 _returnvalue_7 _returnvalue_9) (Variables|/Game/Blueprints/Player/PlayerStateBP.PlayerStateBP_C|GetHighScore _gamestate))
            (else
              (return false 0.0 0.0 0 0 0 0 0 0 (Variables|/Game/Blueprints/Player/PlayerStateBP.PlayerStateBP_C|GetHighScore _gamestate)))))))))

(fn IsGameActive
  (bind _gamestate (Helpers|GetHideandSeekGameState))
  (Utilities|IsValid _gamestate
    (:Is%20Valid
      (return (Variables|/Script/TheLookout.TheLookoutGameStateBase|GetGameActive _gamestate)))
    (:Is%20Not%20Valid
      (return false))))

(fn GetDefaultPawnClassforController
  (params (InController :type Controller%20Object%20Reference))
  (bind _asplayer_controller (Utilities|Casting|CastToPlayerController InController))
  (Class|TurnBasedBlueprintLibrary|GetMyPlayerIndex _asplayer_controller)
  (switch int (Class|GameplayStatics|GetPlayerControllerID _asplayer_controller)
    (:Default
      _)
    (:0
      _))
  (return 0))

(fn SpawnPlayers
  (params (NewPlayerController :type Player%20Controller%20Object%20Reference))
  (Utilities|FlowControl|Sequence
    (:then_0
      (bind _outactors (Actor|GetAllActorsOfClass "/Script/Engine.PlayerStart"))
      (for _array_element _outactors
        (if (Utilities|String|Contains (Utilities|String|ToString(Name) (Variables|/Script/Engine.PlayerStart|GetPlayerStartTag _array_element)) "VR")
          (LocalVariables|SetVRPlayerStart _array_element)
          (else
            (Utilities|Array|Add (LocalVariables|GetRemotePlayerStarts) _array_element)))))
    (:then_1
      (bind _returnvalue (Game|SpawnActorfromClass (Utilities|Select :Index (Variables|Default|GetPlayerIndex) :Option%200 "/Game/Blueprints/Player/VRLookoutPawnBP.VRLookoutPawnBP_C" :Option%201 "/Game/Blueprints/Player/AgentCharacterBP.AgentCharacterBP_C" :Option%202 "/Game/Blueprints/Player/AgentCharacterBP.AgentCharacterBP_C" :Option%203 "/Game/Blueprints/Player/AgentCharacterBP.AgentCharacterBP_C") (Utilities|Select :Index (Variables|Default|GetPlayerIndex) :Option%200 (Transformation|GetActorTransform (LocalVariables|GetVRPlayerStart)) :Option%201 (Transformation|GetActorTransform (Utilities|Array|Get(acopy) (LocalVariables|GetRemotePlayerStarts))) :Option%202 (Transformation|GetActorTransform (Utilities|Array|Get(acopy) (LocalVariables|GetRemotePlayerStarts) 1)) :Option%203 (Transformation|GetActorTransform (Utilities|Array|Get(acopy) (LocalVariables|GetRemotePlayerStarts) 2))) "Undefined" 0 0))
      (bind _aspawn (Utilities|Casting|CastToPawn _returnvalue))
      (Pawn|Possess NewPlayerController _aspawn)
      (bind _result (Math|Integer|IncrementInt (Variables|Default|GetPlayerIndex))
        (:%20%20
          (Variables|Default|SetPlayerIndex _result))))))