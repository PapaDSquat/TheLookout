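; Game state for a hide-and-seek mode that runs a timed round and tracks whether one is active or was just played.
; RestartGame records the duration and start time, while EndGame closes the round, each firing an event dispatcher.
; Tick recomputes the clamped remaining time while active and fires the time-out dispatcher at zero, without ending the round itself.
; A helper returns player 0's PlayerStateBP through the pawn.
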(event EventBeginPlay)

(event EventTick
  (params (DeltaSeconds :type Float%20%28single-precision%29))
  (if (Variables|Default|GetGameActive)
    (bind _timeremaining (Time|UpdateTimeRemaining))
    (if (<= _timeremaining 0.0)
      (Default|CallOnTimeRunOut))))

(fn ConstructionScript)

(fn RestartGame
  (params (GameTimeSeconds :type Float%20%28single-precision%29))
  (Utilities|FlowControl|Sequence
    (:then_0
      (Variables|Time|SetGameTimeTotal GameTimeSeconds)
      (Variables|Time|SetGameTimeAtStartSeconds (Utilities|Time|GetGameTimeinSeconds))
      (Variables|Time|SetTimeRemaining 0.0))
    (:then_1
      (Variables|Default|SetGameJustPlayed false)
      (Variables|Default|SetGameActive true)
      (Default|CallOnGameStart))))

(fn EndGame
  (Variables|Default|SetGameActive false)
  (Variables|Default|SetGameJustPlayed true)
  (Default|CallOnGameEnd))

(fn UpdateTimeRemaining
  (LocalVariables|SetLElapsedTime (- (Utilities|Time|GetGameTimeinSeconds) (Variables|Time|GetGameTimeAtStartSeconds)))
  (bind _output_get (Variables|Time|SetTimeRemaining (Math|Float|Max(Float) (- (Variables|Time|GetGameTimeTotal) (LocalVariables|GetLElapsedTime)) 0.0)))
  (return _output_get))

(fn GetHideandSeekPlayerState
  (bind _returnvalue (Game|Player|GetPlayerPawn 0))
  (Utilities|IsValid _returnvalue
    (:Is%20Valid
      (bind _asplayer_state_bp (Utilities|Casting|CastToPlayerStateBP (Variables|/Script/Engine.Pawn|GetPlayerState _returnvalue))
        (:then
          (return _asplayer_state_bp))
        (:CastFailed
          _)))
    (:Is%20Not%20Valid
      _))
  (return 0))