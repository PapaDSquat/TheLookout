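; VR pawn Blueprint for the lookout player in a hide-and-seek game.
; The StartGame input action fetches the HideAndSeekGameMode and, if it is valid, calls its StartGame.
; Helper functions return the cast game mode and game state, though only the game mode one is used here.
; Left and right hand grab events are empty stubs, with a TODO noted.
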(event Custom|CallGrabRightHand_Pressed
  ;[1 1 1] TODO
)

(event Custom|CallGrabLeftHand_Pressed
  ;[1 1 1] TODO
)

(event EventBeginPlay)

(event Collision|EventActorBeginOverlap
  (params (OtherActor :type Actor%20Object%20Reference)))

(event EventTick
  (params (DeltaSeconds :type Float%20%28single-precision%29)))

(event Input|ActionEvents|InputActionStartGame
  (params (Key :type Key%20Structure :default "None"))
  (bind _gamemode (CallFunction|GetHideandSeekGameMode))
  (:Pressed
    (Utilities|IsValid _gamemode
      (:Is%20Valid
        (Default|StartGame _gamemode)))))

(fn ConstructionScript)

(fn GetHideandSeekGameState
  (bind _ashide_and_seek_game_state (Utilities|Casting|CastToHideAndSeekGameState (Game|GetGameState))
    (:then
      (return _ashide_and_seek_game_state))
    (:CastFailed
      (return 0))))

(fn GetHideandSeekGameMode
  (bind _ashide_and_seek_game_mode (Utilities|Casting|CastToHideAndSeekGameMode (Game|GetGameMode))
    (:then
      (return _ashide_and_seek_game_mode))
    (:CastFailed
      (return 0))))