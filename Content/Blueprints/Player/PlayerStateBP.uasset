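; Player state Blueprint that tracks the player's points, thrown balls, final game score and a persistent high score.
; On BeginPlay it loads the HideAndSeekHighScore save from its slot, or creates a new save object if none exists, and caches the high score.
; Small functions increment or reset the per-game stats, and setting a final score above the high score writes it back to the save slot.
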(event EventBeginPlay
  ;[1 1 1] Create Save Game
  (bind _returnvalue (SaveGame|DoesSaveGameExist (Variables|Default|GetSaveGameName)))
  (if _returnvalue
    (bind _returnvalue_2 (SaveGame|LoadGamefromSlot (Variables|Default|GetSaveGameName)))
    (bind _ashide_and_seek_high_score (Utilities|Casting|CastToHideAndSeekHighScore _returnvalue_2))
    (bind _output_get (Variables|Default|SetSaveGameRef _ashide_and_seek_high_score))
    (Variables|Default|SetHighScore (Variables|/Game/Blueprints/GameMode/HideAndSeekHighScore.HideAndSeekHighScore_C|GetHighScore _output_get))
    (else
      (bind _returnvalue_3 (SaveGame|CreateSaveGameObject "/Game/Blueprints/GameMode/HideAndSeekHighScore.HideAndSeekHighScore_C"))
      (bind _output_get_2 (Variables|Default|SetSaveGameRef _returnvalue_3))
      (Variables|Default|SetHighScore (Variables|/Game/Blueprints/GameMode/HideAndSeekHighScore.HideAndSeekHighScore_C|GetHighScore _output_get_2)))))

(fn ConstructionScript)

(fn ScorePoint
  (Math|Integer|IncrementInt (Variables|Default|GetGamePoints)
    (:%20%20
      (return (Variables|Default|GetGamePoints)))))

(fn ResetGameStats
  (Variables|Default|SetGamePoints 0)
  (Variables|Default|SetGameScore 0)
  (Variables|Default|SetBallsThrown 0))

(fn OnThrowBall
  (Math|Integer|IncrementInt (Variables|Default|GetBallsThrown)))

(fn SetFinalGameScore
  (params (FInalScore :type Integer))
  (bind _output_get (Variables|Default|SetGameScore FInalScore))
  (if (> _output_get (Variables|Default|GetHighScore))
    (CallFunction|SaveHighScore _output_get)))

(fn SaveHighScore
  (params (HighScore :type Integer))
  (bind _savegameref (Variables|Default|GetSaveGameRef))
  (bind _output_get (Variables|Default|SetHighScore HighScore))
  (Utilities|IsValid _savegameref
    (:Is%20Valid
      (Variables|/Game/Blueprints/GameMode/HideAndSeekHighScore.HideAndSeekHighScore_C|SetHighScore _savegameref _output_get)
      (SaveGame|SaveGametoSlot _savegameref (Variables|Default|GetSaveGameName)))))